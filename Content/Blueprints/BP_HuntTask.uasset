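; Behavior tree task that makes a hunter AI move its pawn to the actor stored in the Target blackboard key.
; On execute it casts the owner to BP_HunterController and caches it when no controller is stored yet, then runs AIMoveTo on the controlled pawn.
; The task finishes successfully when the move succeeds; a failed move or failed cast never calls FinishExecute.
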(event `self.ReceiveExecute`
  (params (OwnerActor :type "Actor Object Reference"))
  (if (not (!= (`self.AI_Controller`) null))
    (bind _asbp_hunter_controller (cast `/Game/Blueprints/BP_HunterController` OwnerActor))
    (set `self.AI_Controller` _asbp_hunter_controller))
  (`|AIMoveTo` (`Controller.K2_GetPawn` (`self.AI_Controller`)) (0.0 0.0 0.0) (`BTFunctionLibrary.GetBlackboardValueAsActor` (`self.Target`))
    (:`OnSuccess`
      (`self.FinishExecute` true))))